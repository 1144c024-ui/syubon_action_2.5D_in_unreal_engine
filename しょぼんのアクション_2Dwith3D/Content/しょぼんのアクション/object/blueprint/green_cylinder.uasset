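; Green pipe actor that marks when the BP_syobon character is in position to enter it.
; Overlapping its trigger volume caches the character, sets its CanEnterPipe flag and registers this pipe as its CurrentPipe; leaving clears both on the character.
; The IA_down input handler only validity-checks the cached character, so no entry action happens in this Blueprint.
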(event OnComponentEndOverlap(triggervolume)
  (params (OverlappedComponent :type Primitive%20Component%20Object%20Reference) (OtherActor :type Actor%20Object%20Reference) (OtherComp :type Primitive%20Component%20Object%20Reference) (OtherBodyIndex :type Integer))
  (bind _asbp_syobon (Utilities|Casting|CastToBP_syobon OtherActor))
  (Variables|/Game/しょぼんのアクション/player/Blue_print/BP_syobon.BP_syobon_C|Setcan%20enter%20pipe _asbp_syobon false)
  (Variables|/Game/しょぼんのアクション/player/Blue_print/BP_syobon.BP_syobon_C|Setcurrent%20pipe _asbp_syobon 0))

(event OnComponentBeginOverlap(triggervolume)
  (params (OverlappedComponent :type Primitive%20Component%20Object%20Reference) (OtherActor :type Actor%20Object%20Reference) (OtherComp :type Primitive%20Component%20Object%20Reference) (OtherBodyIndex :type Integer) (bFromSweep :type Boolean) (SweepResult :type Hit%20Result%20Structure%20%28by%20ref%29))
  (bind _asbp_syobon (Utilities|Casting|CastToBP_syobon OtherActor))
  (Variables|Default|Setbp%20syobon _asbp_syobon)
  (bind _output_get (Variables|/Game/しょぼんのアクション/player/Blue_print/BP_syobon.BP_syobon_C|Setcan%20enter%20pipe _asbp_syobon true))
  (if _output_get
    (bind _output_get_2 (Variables|/Game/しょぼんのアクション/player/Blue_print/BP_syobon.BP_syobon_C|Setcurrent%20pipe _asbp_syobon self))
    (Utilities|IsValid _output_get_2)))

(event Input|EnhancedActionEvents|EnhancedInputActionIA_down
  (params (ActionValue :type Boolean) (ElapsedSeconds :type Float%20%28double-precision%29) (TriggeredSeconds :type Float%20%28double-precision%29) (InputAction :type Input%20Action%20Object%20Reference :default "/Game/oldthing/ThirdPerson/Input/Actions/IA_down.IA_down"))
  (Utilities|IsValid (Variables|Default|Getbp%20syobon)))

(fn ConstructionScript)