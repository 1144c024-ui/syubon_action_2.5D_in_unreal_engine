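; BP_final_Goal is a goal trigger in the Syobon Action game that ends a level and loads the next one.
; When BP_syobon overlaps its Box, it stores the character and its location, then plays the goal sound.
; Tick moves the character back to that stored location every frame, holding it in place.
; After a ten-second delay, it opens the level named by its NextLevel variable.
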(event OnComponentBeginOverlap(Box)
  (params (OverlappedComponent :type Primitive%20Component%20Object%20Reference) (OtherActor :type Actor%20Object%20Reference) (OtherComp :type Primitive%20Component%20Object%20Reference) (OtherBodyIndex :type Integer) (bFromSweep :type Boolean) (SweepResult :type Hit%20Result%20Structure%20%28by%20ref%29))
  (bind _asbp_syobon (Utilities|Casting|CastToBP_syobon OtherActor))
  (bind _output_get (Variables|Default|Setsyobon _asbp_syobon))
  (Variables|Default|SetNewVar (Transformation|GetActorLocation _output_get))
  (Audio|PlaySound2D "/Game/しょぼんのアクション/object/sound_effect/ゴール.ゴール" 1.0 1.0 0.0 0 0)
  (Utilities|FlowControl|Delay 1e+01)
  (Game|OpenLevel(byName) (Utilities|String|StringToName (Variables|Default|GetNextLevel))))

(event EventTick
  (params (DeltaSeconds :type Float%20%28single-precision%29))
  (bind _syobon (Variables|Default|Getsyobon))
  (Utilities|IsValid _syobon
    (:Is%20Valid
      (Transformation|SetActorLocation _syobon (Variables|Default|GetNewVar) false false))))

(fn ConstructionScript)