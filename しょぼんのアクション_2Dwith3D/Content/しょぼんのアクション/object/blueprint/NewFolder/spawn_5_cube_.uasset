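; A trigger actor for the Syobon Action game that springs a row of Quation_cube_hide_ blocks when the player character BP_syobon enters it.
; Overlap on component R fires once through a DoOnce, which any non-player overlap resets.
; After a short delay, a loop spawns seven evenly spaced cubes along X, slightly above the actor and centered on it, despite the "5" in the asset name.
; It prints a debug string per cube, then destroys itself.
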(event OnComponentBeginOverlap(r)
  (params (OverlappedComponent :type Primitive%20Component%20Object%20Reference) (OtherActor :type Actor%20Object%20Reference) (OtherComp :type Primitive%20Component%20Object%20Reference) (OtherBodyIndex :type Integer) (bFromSweep :type Boolean) (SweepResult :type Hit%20Result%20Structure%20%28by%20ref%29))
  (bind _returnvalue (Transformation|GetActorLocation))
  (Utilities|Casting|CastToBP_syobon OtherActor
    (:then
      (Utilities|FlowControl|DoOnce false :!label _label
        (:Completed
          (Utilities|FlowControl|Delay 0.5)
          (for _index (range -3 3)
            (bind _output_get (Variables|Default|SetNewVar (* _index 100)))
            (Game|SpawnActorfromClass "/Game/しょぼんのアクション/object/blueprint/QUATION_CUBE_FAMILLY/quation_cube_hide_.quation_cube_hide__C" (Math|Transform|MakeTransform (Math|Vector|MakeVector (+ _output_get (.x _returnvalue)) (.y _returnvalue) (+ (.z _returnvalue) 4e+01)) "0, 0, 0" "1.000000,1.000000,1.000000") "Undefined" "MultiplyWithRoot" 0 0)
            (Development|PrintString "Hello"))
          (Actor|DestroyActor))))
    (:CastFailed
      (goto _label Reset))))

(fn ConstructionScript)