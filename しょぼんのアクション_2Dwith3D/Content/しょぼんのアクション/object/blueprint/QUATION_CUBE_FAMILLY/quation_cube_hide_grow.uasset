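; A hidden question block for a Syobon Action-style game that reveals itself when BP_syobon overlaps its underside trigger.
; On the first such overlap only, it makes the mesh visible and blocking, plays the coin sound and spawns a grow mushroom above itself.
; After a short delay it swaps the mesh to a static material, marking the block as used.
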(event OnComponentBeginOverlap(under_hit)
  (params (OverlappedComponent :type Primitive%20Component%20Object%20Reference) (OtherActor :type Actor%20Object%20Reference) (OtherComp :type Primitive%20Component%20Object%20Reference) (OtherBodyIndex :type Integer) (bFromSweep :type Boolean) (SweepResult :type Hit%20Result%20Structure%20%28by%20ref%29))
  (bind _returnvalue (Transformation|GetActorLocation))
  (bind _staticmesh (Variables|Default|GetStaticMesh))
  (Utilities|Casting|CastToBP_syobon OtherActor)
  (Utilities|FlowControl|DoOnce false
    (:Completed
      (Rendering|SetVisibility (Variables|Default|GetStaticMesh) true false)
      (Collision|SetCollisionResponsetoAllChannels _staticmesh "ECR_Block")
      (Audio|PlaySound2D "/Game/しょぼんのアクション/object/sound_effect/coin.coin" 1.0 1.0 0.0 0 0)
      (Game|SpawnActorfromClass "/Game/しょぼんのアクション/object/blueprint/mashroom_grow.mashroom_grow_C" (Math|Transform|MakeTransform (Math|Vector|MakeVector (.x _returnvalue) (.y _returnvalue) (+ (.z _returnvalue) 1e+02)) "0, 0, 0" "1.000000,1.000000,1.000000") "Undefined" "MultiplyWithRoot" 0 0)
      (Utilities|FlowControl|Delay 0.2)
      (Rendering|Material|SetMaterial _staticmesh 0 "/Game/しょぼんのアクション/object/MODEL/material/STATTIC1.STATTIC1"))))

(fn ConstructionScript)