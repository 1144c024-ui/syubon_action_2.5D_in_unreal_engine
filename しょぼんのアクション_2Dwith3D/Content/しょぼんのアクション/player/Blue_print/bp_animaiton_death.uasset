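; Death animation actor for the player in the Syobon Action game, which moves itself along a vertical offset from its owner SyobonOwner.
; On BeginPlay the DEATH timeline starts, and each update adds its Yyy track to the owner's current Z.
; The first valid update spawns a Spawn_font_system actor as TextOwner after the move steps, so TextOwner is still unset when first moved.
; Later updates move that text actor to the same position.
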(event EventBeginPlay
  (bind _syobon_owner (Variables|Default|Getsyobon_owner))
  (Utilities|FlowControl|Delay 0.0)
  (bind _yyy (Timeline|DEATH Play)
    (:Update
      (Utilities|IsValid _syobon_owner
        (:Is%20Valid
          (Variables|Default|SetVECTOR_ORIN (Transformation|GetActorLocation _syobon_owner))
          (Utilities|FlowControl|Sequence
            (:then_0
              (Transformation|SetActorLocation (Math|Vector|MakeVector (.x (Variables|Default|GetVECTOR_ORIN)) (.y (Variables|Default|GetVECTOR_ORIN)) (+ (.z (Variables|Default|GetVECTOR_ORIN)) _yyy)) false false))
            (:then_1
              (Utilities|IsValid (Variables|Default|Getsyobon_owner)
                (:Is%20Valid
                  (Transformation|SetActorLocation (Variables|Default|Gettext_owner) (Math|Vector|MakeVector (.x (Variables|Default|GetVECTOR_ORIN)) (.y (Variables|Default|GetVECTOR_ORIN)) (+ (.z (Variables|Default|GetVECTOR_ORIN)) _yyy)) false false))))
            (:then_2
              (Utilities|FlowControl|DoOnce false
                (:Completed
                  (bind _returnvalue (Game|SpawnActorfromClass "/Game/しょぼんのアクション/player/Blue_print/spawn_font_system.spawn_font_system_C" (Math|Transform|MakeTransform (Variables|Default|GetVECTOR_ORIN) "0, 0, 0" "1.000000,1.000000,1.000000") "Undefined" "MultiplyWithRoot" 0 0))
                  (Variables|Default|Settext_owner _returnvalue))))))))))

(fn ConstructionScript)