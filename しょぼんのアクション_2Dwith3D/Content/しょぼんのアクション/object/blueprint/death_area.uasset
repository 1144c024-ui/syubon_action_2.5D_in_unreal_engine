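; Death area is a moving hazard in a Syobon Action game that kills the player character, BP_syobon, on contact.
; It feeds its Diriction value into movement input every tick to travel along the X axis.
; When its Cube overlaps BP_syobon, it calls Death once and disables its own collision.
; Any other overlap flips the direction and turns the actor 180 degrees in yaw.
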(event OnComponentBeginOverlap(cube)
  (params (OverlappedComponent :type Primitive%20Component%20Object%20Reference) (OtherActor :type Actor%20Object%20Reference) (OtherComp :type Primitive%20Component%20Object%20Reference) (OtherBodyIndex :type Integer) (bFromSweep :type Boolean) (SweepResult :type Hit%20Result%20Structure%20%28by%20ref%29))
  (bind _asbp_syobon (Utilities|Casting|CastToBP_syobon OtherActor)
    (:then
      (Utilities|FlowControl|DoOnce false
        (:Completed
          (Utilities|FlowControl|Sequence
            (:then_0
              (Default|Death? _asbp_syobon)
              (Collision|SetActorEnableCollision false))))))
    (:CastFailed
      (Variables|Default|Setdiriction (* (Variables|Default|Getdiriction) -1.0))
      (Transformation|SetActorRotation (Math|Rotator|MakeRotator 0.0 0.0 (+ (.yaw (Transformation|GetActorRotation)) 1.8e+02))))))

(event EventTick
  (params (DeltaSeconds :type Float%20%28single-precision%29))
  (Pawn|Input|AddMovementInput (Math|Vector|MakeVector (Variables|Default|Getdiriction) 0.0 0.0) 1.0 false))

(fn ConstructionScript)