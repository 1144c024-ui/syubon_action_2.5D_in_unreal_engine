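; Cloud object for a Syobon Action level that moves vertically while the BP_syobon character overlaps its Under_hit component.
; On BeginPlay it stores its origin, and overlap begin plays a Timeline whose curve is added to the origin Z each update, leaving X and Y fixed.
; Overlap end stops the Timeline after a short delay without resetting, so the cloud stays at its current height.
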(event OnComponentBeginOverlap(under_hit)
  (params (OverlappedComponent :type Primitive%20Component%20Object%20Reference) (OtherActor :type Actor%20Object%20Reference) (OtherComp :type Primitive%20Component%20Object%20Reference) (OtherBodyIndex :type Integer) (bFromSweep :type Boolean) (SweepResult :type Hit%20Result%20Structure%20%28by%20ref%29))
  (Utilities|Casting|CastToBP_syobon OtherActor)
  (CallFunction|PlayAnimaa))

(event OnComponentEndOverlap(under_hit)
  (params (OverlappedComponent :type Primitive%20Component%20Object%20Reference) (OtherActor :type Actor%20Object%20Reference) (OtherComp :type Primitive%20Component%20Object%20Reference) (OtherBodyIndex :type Integer))
  (Utilities|Casting|CastToBP_syobon OtherActor)
  (Utilities|FlowControl|Delay 0.1)
  (CallFunction|StopPlayAnima))

(event Custom|play%20animaa
  (bind _orin_locate (Variables|Default|Getorin_locate))
  (bind _ooo (Timeline|Timeline Play)
    (:Update
      (Transformation|SetActorLocation (Math|Vector|MakeVector (.x _orin_locate) (.y _orin_locate) (+ _ooo (.z _orin_locate))) false false))))

(event Custom|stop%20play%20anima
  (bind _orin_locate (Variables|Default|Getorin_locate))
  (bind _ooo (Timeline|Timeline Stop)
    (:Update
      (Transformation|SetActorLocation (Math|Vector|MakeVector (.x _orin_locate) (.y _orin_locate) (+ _ooo (.z _orin_locate))) false false))))

(event EventBeginPlay
  (Variables|Default|Setorin_locate (Transformation|GetActorLocation)))

(fn ConstructionScript)