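; Player character for a Syobon Action 2D platformer, with Enhanced Input movement and jumping plus flipbook animation.
; BeginPlay briefly shows the death counter, then starts data-table music by level name and enables input, adding an ending widget on "to_be_continued".
; Timeline-driven pipe entry either launches player and pipe together or opens "to_be_continued".
; Death spawns an animation actor, decrements the GameInstance counter and restarts the level after a delay.
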(event Custom|update_animation
  (bind _sprite (Variables|Default|GetSprite))
  (if (AI|Components|NavMovement|IsFalling (Variables|Character|GetCharacterMovement))
    (Sprite|SetFlipbook _sprite "/Game/しょぼんのアクション/player/flip_book/FB_Jump.FB_Jump")
    (Utilities|FlowControl|DoOnce false :!label _label
      (:Completed
        (Audio|PlaySound2D "/Game/しょぼんのアクション/player/sound_effect/ジャンプ_JUMP_.ジャンプ_JUMP_" 1.0 1.0 0.0 0 0)))
    (elif (or (> (.x (Transformation|GetVelocity)) 0.0) (< (.x (Transformation|GetVelocity)) 0.0))
      (Sprite|SetFlipbook _sprite "/Game/しょぼんのアクション/player/flip_book/FB_Walk.FB_Walk")
      (goto _label Reset)
      (else
        (Sprite|SetFlipbook _sprite "/Game/しょぼんのアクション/player/flip_book/FB_Idle.FB_Idle")))))

(event Custom|death?
  (bind _returnvalue (Transformation|GetActorTransform))
  (Utilities|FlowControl|DoOnce false
    (:Completed
      (Audio|Components|Audio|Stop (Variables|Default|Getplay_music))
      (Variables|Default|Setdeath true)
      (Input|DisableInput 0)
      (Collision|SetActorEnableCollision true)
      (Game|SpawnActorfromClass "/Game/しょぼんのアクション/player/Blue_print/bp_animaiton_death.bp_animaiton_death_C" (Math|Transform|MakeTransform (Math|Vector|MakeVector (.x (.location _returnvalue)) (.y (.location _returnvalue)) (.z (.location _returnvalue))) (.rotation _returnvalue) (.scale _returnvalue)) "Undefined" "OverrideRootScale" 0 self 0)
      (Rendering|SetActorHiddenInGame true)
      (Audio|PlaySound2D "/Game/しょぼんのアクション/player/sound_effect/death.death" 1.0 1.0 0.0 0 0)
      (bind _asgi_syobon (Utilities|Casting|CastToGI_syobon (Game|GetGameInstance)))
      (Variables|/Game/しょぼんのアクション/player/Blue_print/GI_syobon.GI_syobon_C|Setdeath_count _asgi_syobon (- (Variables|/Game/しょぼんのアクション/player/Blue_print/GI_syobon.GI_syobon_C|Getdeath_count _asgi_syobon) 1))
      (Utilities|FlowControl|Delay 3.5)
      (Development|ExecuteConsoleCommand "RestartLevel" 0))))

(event Custom|UUU
  (bind _pipe_location (Variables|Default|Getpipe_location))
  (bind _current_location_in_pipe (Variables|Default|Getcurrent_location_in_pipe))
  (bind _newtrack_0 (Timeline|death_pipe Play)
    (:Update
      (Utilities|FlowControl|Sequence
        (:then_0
          (Transformation|SetActorLocation (Math|Vector|MakeVector (.x _current_location_in_pipe) (.y _current_location_in_pipe) (+ (.z _current_location_in_pipe) _newtrack_0)) false false))
        (:then_1
          (Transformation|SetActorLocation (Variables|Default|Getcurrent%20pipe) (Math|Vector|MakeVector (.x _pipe_location) (.y _pipe_location) (+ _newtrack_0 (.z _pipe_location))) false false))))))

(event Input|EnhancedActionEvents|EnhancedInputActionIA_Move
  (params (ActionValue :type Vector%202D%20Structure) (ElapsedSeconds :type Float%20%28double-precision%29) (TriggeredSeconds :type Float%20%28double-precision%29) (InputAction :type Input%20Action%20Object%20Reference :default "/Game/oldthing/ThirdPerson/Input/Actions/IA_Move.IA_Move"))
  (bind _x (Math|Vector2D|BreakVector2D ActionValue))
  (bind _sprite (Variables|Default|GetSprite))
  (Pawn|Input|AddMovementInput "1.000000,0.000000,0.000000" _x false)
  (Math|Float|CompareFloat _x 0.0
    (:>
      (Transformation|SetRelativeRotation _sprite "0, 0, 0" false false))
    (:<
      (Transformation|SetRelativeRotation _sprite "0.000000,180.000000,0.000000" false false))))

(event Input|EnhancedActionEvents|EnhancedInputActionIA_Jump
  (params (ActionValue :type Vector%202D%20Structure) (ElapsedSeconds :type Float%20%28double-precision%29) (TriggeredSeconds :type Float%20%28double-precision%29) (InputAction :type Input%20Action%20Object%20Reference :default "/Game/oldthing/ThirdPerson/Input/Actions/IA_Jump.IA_Jump"))
  (:Triggered
    (Character|Jump))
  (:Completed
    (Character|StopJumping)))

(event Input|EnhancedActionEvents|EnhancedInputActionIA_down
  (params (ActionValue :type Boolean) (ElapsedSeconds :type Float%20%28double-precision%29) (TriggeredSeconds :type Float%20%28double-precision%29) (InputAction :type Input%20Action%20Object%20Reference :default "/Game/oldthing/ThirdPerson/Input/Actions/IA_down.IA_down"))
  (if (Variables|Default|Getcan%20enter%20pipe)
    (Utilities|IsValid (Variables|Default|Getcurrent%20pipe_0)
      (:Is%20Valid
        (Input|DisableInput 0)
        (Variables|Default|Setcurrent_location_in_pipe (Transformation|GetActorLocation))
        (Audio|PlaySound2D "/Game/しょぼんのアクション/object/sound_effect/土管_水管TP_.土管_水管TP_" 1.0 1.0 0.0 0 0)
        (bind _newtrack_0 (Timeline|Timeline Play)
          (:Update
            (Transformation|SetActorLocation (Math|Vector|MakeVector (.x (Variables|Default|Getcurrent_location_in_pipe)) (.y (Variables|Default|Getcurrent_location_in_pipe)) (+ (.z (Variables|Default|Getcurrent_location_in_pipe)) _newtrack_0)) false false))
          (:Finished
            (Variables|Default|Setcurrent_location_in_pipe (Transformation|GetActorLocation))
            (Variables|Default|Setpipe_location (Transformation|GetActorLocation (Variables|Default|Getcurrent%20pipe_0)))
            (Game|OpenLevel(byName) "to_be_continued")))))))

(event Input|EnhancedActionEvents|EnhancedInputActionIA_down
  (params (ActionValue :type Boolean) (ElapsedSeconds :type Float%20%28double-precision%29) (TriggeredSeconds :type Float%20%28double-precision%29) (InputAction :type Input%20Action%20Object%20Reference :default "/Game/oldthing/ThirdPerson/Input/Actions/IA_down.IA_down"))
  (if (Variables|Default|Getcan%20enter%20pipe)
    (Utilities|IsValid (Variables|Default|Getcurrent%20pipe)
      (:Is%20Valid
        (Input|DisableInput 0)
        (Variables|Default|Setcurrent_location_in_pipe (Transformation|GetActorLocation))
        (Audio|PlaySound2D "/Game/しょぼんのアクション/object/sound_effect/土管_水管TP_.土管_水管TP_" 1.0 1.0 0.0 0 0)
        (bind _newtrack_0 (Timeline|pipe Play)
          (:Update
            (Transformation|SetActorLocation (Math|Vector|MakeVector (.x (Variables|Default|Getcurrent_location_in_pipe)) (.y (Variables|Default|Getcurrent_location_in_pipe)) (+ (.z (Variables|Default|Getcurrent_location_in_pipe)) _newtrack_0)) false false))
          (:Finished
            (Variables|Default|Setcurrent_location_in_pipe (Transformation|GetActorLocation))
            (Variables|Default|Setpipe_location (Transformation|GetActorLocation (Variables|Default|Getcurrent%20pipe)))
            (CallFunction|UUU)))))))

(event EventTick
  (params (DeltaSeconds :type Float%20%28single-precision%29))
  (if (not (Variables|Default|Getdeath))
    (CallFunction|UpdateAnimation)
    (if (> (Variables|Default|GetGRAVITY_CUST) 0)
      (Sprite|SetFlipbook (Variables|Default|GetSprite) "/Game/しょぼんのアクション/player/flip_book/NewPaperFlipbook.NewPaperFlipbook"))))

(event EventBeginPlay
  (Utilities|FlowControl|FlipFlop :!label _label
    (:A
      (bind _returnvalue (UserInterface|CreateWidget "/Game/しょぼんのアクション/player/icon/death_count.death_count_C"))
      (UserInterface|Viewport|AddtoViewport _returnvalue 0)
      (Utilities|FlowControl|Delay 2.0)
      (goto _label))
    (:B
      (Widget|RemovefromParent _returnvalue)
      (bind _returnvalue_2 (Game|GetCurrentLevelName true))
      (bind _returnvalue_3 (Utilities|GetDataTableRow "/Game/しょぼんのアクション/player/Blue_print/music.music" (Utilities|String|StringToName _returnvalue_2))
        (:then
          (bind _returnvalue_4 (Audio|SpawnSound2D (Utilities|Struct|Breakstructure_muisc _returnvalue_3) 1.0 1.0 0.0 0))
          (Variables|Default|Setplay_music _returnvalue_4)
          (Utilities|FlowControl|Sequence
            (:then_0
              (bind _asplayer_controller (Utilities|Casting|CastToPlayerController (Pawn|GetController)))
              (Input|AddMappingContext (PlayerController|LocalPlayerSubsystems|GetEnhancedInputLocalPlayerSubsystem _asplayer_controller) "/Game/oldthing/ThirdPerson/Input/IMC_Default.IMC_Default" 0 "(bIgnoreAllPressedKeysUntilRelease=True,bForceImmediately=False,bNotifyUserSettings=False)"))
            (:then_1
              (if (== "to_be_continued" (Utilities|String|StringToName _returnvalue_2))
                (Utilities|FlowControl|Delay 3.5)
                (bind _returnvalue_5 (UserInterface|CreateWidget "/Game/しょぼんのアクション/map/to_be_cotinued_widget.to_be_cotinued_widget_C"))
                (UserInterface|Animation|PlayAnimation _returnvalue_5 (Variables|/Game/しょぼんのアクション/map/to_be_cotinued_widget.to_be_cotinued_widget_C|Getto_be_continued _returnvalue_5) 0.0 1 "Forward" 1.0 false)
                (UserInterface|Viewport|AddtoViewport _returnvalue_5 0)))))))))

(fn ConstructionScript)