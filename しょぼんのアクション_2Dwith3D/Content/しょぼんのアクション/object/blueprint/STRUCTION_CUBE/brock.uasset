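; Breakable brick block for the Syobon Action game that shatters after BP_syobon touches it.
; Overlapping the Box with BP_syobon latches TOUCHED, which is never cleared.
; Tick then polls the player's GRAVITYCUST through a DoOnce that resets until the value is positive.
; At that point the block plays a break sound, spawns a scaled-up Niagara brick effect and destroys itself.
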(event OnComponentBeginOverlap(Box)
  (params (OverlappedComponent :type Primitive%20Component%20Object%20Reference) (OtherActor :type Actor%20Object%20Reference) (OtherComp :type Primitive%20Component%20Object%20Reference) (OtherBodyIndex :type Integer) (bFromSweep :type Boolean) (SweepResult :type Hit%20Result%20Structure%20%28by%20ref%29))
  (Utilities|Casting|CastToBP_syobon OtherActor)
  (Variables|Default|SetTOUCHED true))

(event EventBeginPlay)

(event Collision|EventActorBeginOverlap
  (params (OtherActor :type Actor%20Object%20Reference)))

(event EventTick
  (params (DeltaSeconds :type Float%20%28single-precision%29))
  (if (Variables|Default|GetTOUCHED)
    (Utilities|FlowControl|DoOnce false :!label _label
      (:Completed
        (bind _returnvalue (Actor|GetActorOfClass "/Game/しょぼんのアクション/player/Blue_print/BP_syobon.BP_syobon_C"))
        (if (> (Variables|/Game/しょぼんのアクション/player/Blue_print/BP_syobon.BP_syobon_C|GetGRAVITY_CUST _returnvalue) 0)
          (Audio|PlaySound2D "/Game/しょぼんのアクション/object/sound_effect/break_rock.break_rock" 1.0 1.0 0.0 0 0)
          (Niagara|SpawnSystematLocation "/Game/Generic_Item_Destruction_FX/Visual_Effects/NiagaraSystem/NS_Brick.NS_Brick" (Transformation|GetActorLocation) "0, 0, 0" "8.000000,8.000000,8.000000")
          (Actor|DestroyActor)
          (else
            (goto _label Reset)))))))

(fn ConstructionScript)